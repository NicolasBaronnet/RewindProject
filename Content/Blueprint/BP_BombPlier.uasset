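; BP_BombPlier is a pliers tool for the motion controller pawn that picks up and carries a bomb's core.
; Its sphere records an overlapping BP_CoreBomb, which StartUse attaches to the pliers and StopUse detaches.
; Tick also detaches the overlapped actor while the cached BP_Timer's rewind state is set.
; GetSocketName picks the left or right pliers socket from the pawn's GrabLeft state.
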(event OnComponentBeginOverlap(Sphere)
  (params (OverlappedComponent :type Primitive%20Component%20Object%20Reference) (OtherActor :type Actor%20Object%20Reference) (OtherComp :type Primitive%20Component%20Object%20Reference) (OtherBodyIndex :type Integer) (bFromSweep :type Boolean) (SweepResult :type Hit%20Result%20Structure%20%28by%20ref%29))
  (if (== (Utilities|GetClass OtherActor) "/Game/Blueprint/BP_CoreBomb.BP_CoreBomb_C")
    (Variables|Default|SetOverlappedActorRef OtherActor)
    (Variables|Default|SetOverlappedCompRef OtherComp)))

(event EventBeginPlay
  (|CallParentFunction)
  (bind _asbp_bomb (Utilities|Casting|CastToBP_BombClass "/Game/Blueprint/BP_Bomb.BP_Bomb_C"))
  (Actor|GetActorOfClass _asbp_bomb)
  (bind _asbp_timer (Utilities|Casting|CastToBP_TimerClass "/Game/Blueprint/BP_Timer.BP_Timer_C"))
  (bind _returnvalue (Actor|GetActorOfClass _asbp_timer))
  (Variables|Default|SetTimerRef_0 _returnvalue))

(event Collision|EventActorBeginOverlap
  (params (OtherActor :type Actor%20Object%20Reference))
  (|CallParentFunction OtherActor) ; This node is disabled and will not be called.\nDrag off pins to build functionality.
)

(event EventTick
  (params (DeltaSeconds :type Float%20%28single-precision%29))
  (bind _timerref_0 (Variables|Default|GetTimerRef_0))
  (|CallParentFunction DeltaSeconds)
  (Utilities|IsValid _timerref_0
    (:Is%20Valid
      (if (Variables|/Game/Blueprint/BP_Timer.BP_Timer_C|GetRewindStateRef _timerref_0)
        (Utilities|IsValid (Variables|Default|GetOverlappedActorRef)
          (:Is%20Valid
            (Transformation|DetachFromActor (Variables|Default|GetOverlappedActorRef) "KeepRelative" "KeepRelative" "KeepRelative")))))))

(event EventStartUse
  (bind _overlappedactorref (Variables|Default|GetOverlappedActorRef))
  (bind _asbp_core_bomb (Utilities|Casting|CastToBP_CoreBombClass "/Game/Blueprint/BP_CoreBomb.BP_CoreBomb_C"))
  (bind _returnvalue (Actor|GetActorOfClass _asbp_core_bomb))
  (if (== _returnvalue _overlappedactorref)
    (Transformation|AttachActorToActor _overlappedactorref self "None" "KeepWorld" "KeepWorld" "KeepWorld" true)))

(event EventStopUse
  (Utilities|IsValid (Variables|Default|GetOverlappedActorRef)
    (:Is%20Valid
      (Transformation|DetachFromActor (Variables|Default|GetOverlappedActorRef) "KeepRelative" "KeepRelative" "KeepRelative"))))

(fn ConstructionScript
  (|CallParentFunction))

(fn GetSocketName
  (bind _asmotion_controller_pawn (Utilities|Casting|CastToMotionControllerPawn (Game|Player|GetPlayerPawn 0)))
  (if (Variables|/Game/Blueprint/MotionControllerPawn.MotionControllerPawn_C|GetGrabLeft _asmotion_controller_pawn)
    (LocalVariables|SetSocketName (Utilities|String|StringToName (Utilities|String|Append "TakeBombPlier" "_L")))
    (else
      (LocalVariables|SetSocketName (Utilities|String|StringToName (Utilities|String|Append "TakeBombPlier" "_R")))))
  (return (LocalVariables|GetSocketName)))