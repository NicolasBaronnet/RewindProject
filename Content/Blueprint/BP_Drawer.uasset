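; BP_Drawer is a grabbable drawer that slides along world Y as it follows the hand component holding it.
; BeginPlay derives the travel limits from two spline points, and Tick moves the mesh with an offset until release or until the hand leaves that range.
; One drawer type always moves when grabbed, while another moves only once unlocked through an event bound to the referenced color panel.
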(event Custom|UnlockDrawer
  (Variables|Default|SetIsLocked? false))

(event EventBeginPlay
  (bind _colorpanelref (Variables|Default|GetColorPanelRef))
  (|CallParentFunction)
  (Variables|Default|SetStartPoint (Math|Vector|MakeVector 0.0 (+ (.y (Spline|GetLocationatSplinePoint (Variables|Default|GetSpline) 0 "World")) 92.0) 0.0))
  (Variables|Default|SetEndPoint (Math|Vector|MakeVector 0.0 (+ (.y (Spline|GetLocationatSplinePoint (Variables|Default|GetSpline) 1 "World")) 92.0) 0.0))
  (Variables|Default|SetDrawerLocation (Transformation|GetWorldLocation (Variables|Default|GetDefaultSceneRoot)))
  (Utilities|IsValid _colorpanelref
    (:Is%20Valid
      (EventDispatchers|BindEventtoUnlockedDrawer _colorpanelref (delegate Custom|UnlockDrawer)))))

(event Collision|EventActorBeginOverlap
  (params (OtherActor :type Actor%20Object%20Reference)))

(event EventTick
  (params (DeltaSeconds :type Float%20%28single-precision%29))
  (bind _handref (Variables|Default|GetHandRef))
  (bind _drawerlocation (Variables|Default|GetDrawerLocation))
  (|CallParentFunction DeltaSeconds)
  (if (Variables|Default|GetMoving)
    (Utilities|IsValid _handref
      (:Is%20Valid
        (bind _output_get (Variables|Default|SetHandLocation (Transformation|GetWorldLocation _handref)))
        (if (and (< (.y _output_get) (.y (Variables|Default|GetEndPoint))) (> (.y _output_get) (.y (Variables|Default|GetStartPoint))))
          (Transformation|SetWorldLocation (Variables|Default|GetStaticMesh) (Math|Vector|MakeVector (.x _drawerlocation) (+ (.y _output_get) -1.1e+02) (.z _drawerlocation)) false false)
          (else
            (Variables|Default|SetMoving false))))
      (:Is%20Not%20Valid
        (Development|PrintString "Error HandRef")))))

(event EventGrab
  (params (Attach%20to :type Scene%20Component%20Object%20Reference))
  (if (Utilities|Enum|Equal(Enum) (Variables|Default|GetDrawerType) "NewEnumerator0")
    (Variables|Default|SetHandRef Attach%20to)
    (Variables|Default|SetMoving true)
    (else
      (Variables|Default|SetHandRef Attach%20to)
      (if (Utilities|Enum|Equal(Enum) (Variables|Default|GetDrawerType) "NewEnumerator1")
        (if (not (Variables|Default|GetIsLocked?))
          (Variables|Default|SetMoving true))))))

(event EventRelease
  (Variables|Default|SetMoving false)
  (Variables|Default|SetHandRef 0))

(fn ConstructionScript
  (|CallParentFunction))

(fn GetSocketName
  (return "None"))

(fn GrabBehvior
  (return "NewEnumerator1"))