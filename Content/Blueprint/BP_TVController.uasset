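; BP_TVController is a TV remote for use with the motion controller pawn that switches the screen material on a referenced TV.
; StartUse plays a button sound, and nested FlipFlops cycle the screen through four materials on successive presses, with no index variable.
; GetSocketName reads the pawn's GrabLeft flag to return the left or right variant of the TakeTVController socket name.
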(event EventBeginPlay
  (|CallParentFunction) ; This node is disabled and will not be called.\nDrag off pins to build functionality.
)

(event Collision|EventActorBeginOverlap
  (params (OtherActor :type Actor%20Object%20Reference))
  (|CallParentFunction OtherActor) ; This node is disabled and will not be called.\nDrag off pins to build functionality.
)

(event EventTick
  (params (DeltaSeconds :type Float%20%28single-precision%29))
  (|CallParentFunction DeltaSeconds) ; This node is disabled and will not be called.\nDrag off pins to build functionality.
)

(event EventStartUse
  (bind _tvref (Variables|Default|GetTVRef))
  (bind _screen (Variables|/Game/Blueprint/BP_Screen.BP_Screen_C|GetScreen _tvref))
  (Audio|PlaySound2D "/Game/Sounds/Ambiant/bouton.bouton" 1.0 1.0 0.0 0 0)
  (Utilities|FlowControl|FlipFlop
    (:A
      (Utilities|FlowControl|FlipFlop
        (:A
          (Rendering|Material|SetMaterial _screen 0 "/Game/Material/screen_middle/M_MiddleScreenColors.M_MiddleScreenColors"))
        (:B
          (Rendering|Material|SetMaterial _screen 0 "/Game/Material/base_content_material/blinn1.blinn1"))))
    (:B
      (Utilities|FlowControl|FlipFlop
        (:A
          (Rendering|Material|SetMaterial _screen 0 "/Game/import/materials/Jaune.Jaune"))
        (:B
          (Rendering|Material|SetMaterial _screen 0 "/Game/import/desk/Rouge.Rouge"))))))

(fn ConstructionScript
  (|CallParentFunction))

(fn GetSocketName
  (bind _asmotion_controller_pawn (Utilities|Casting|CastToMotionControllerPawn (Game|Player|GetPlayerPawn 0)))
  (if (Variables|/Game/Blueprint/MotionControllerPawn.MotionControllerPawn_C|GetGrabLeft _asmotion_controller_pawn)
    (LocalVariables|SetSocketName (Utilities|String|StringToName (Utilities|String|Append "TakeTVController" "_L")))
    (else
      (LocalVariables|SetSocketName (Utilities|String|StringToName (Utilities|String|Append "TakeTVController" "_R")))))
  (return (LocalVariables|GetSocketName)))