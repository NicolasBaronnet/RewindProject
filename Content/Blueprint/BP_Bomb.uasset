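; Bomb actor that detonates when the level's BP_Timer runs out.
; BeginPlay caches the timer and BP_CoreBomb; the core overlapping any of four trigger boxes sets the time to one second, unless rewinding.
; Tick polls the timer to fire explosion trails and sound through a DoOnce, which resets while time is positive.
; Tick also loops over ScrewArray with an empty body.
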(event OnComponentBeginOverlap(Box)
  (params (OverlappedComponent :type Primitive%20Component%20Object%20Reference) (OtherActor :type Actor%20Object%20Reference) (OtherComp :type Primitive%20Component%20Object%20Reference) (OtherBodyIndex :type Integer) (bFromSweep :type Boolean) (SweepResult :type Hit%20Result%20Structure%20%28by%20ref%29))
  (if (not (Variables|/Game/Blueprint/BP_Timer.BP_Timer_C|GetRewindStateRef (Variables|Default|GetTimerRef)))
    (if (== OtherActor (Variables|Default|GetBombCoreRef))
      (Variables|/Game/Blueprint/BP_Timer.BP_Timer_C|SetTime (Variables|Default|GetTimerRef) 1.0))))

(event OnComponentBeginOverlap(Box1)
  (params (OverlappedComponent :type Primitive%20Component%20Object%20Reference) (OtherActor :type Actor%20Object%20Reference) (OtherComp :type Primitive%20Component%20Object%20Reference) (OtherBodyIndex :type Integer) (bFromSweep :type Boolean) (SweepResult :type Hit%20Result%20Structure%20%28by%20ref%29))
  (if (not (Variables|/Game/Blueprint/BP_Timer.BP_Timer_C|GetRewindStateRef (Variables|Default|GetTimerRef)))
    (if (== OtherActor (Variables|Default|GetBombCoreRef))
      (Variables|/Game/Blueprint/BP_Timer.BP_Timer_C|SetTime (Variables|Default|GetTimerRef) 1.0))))

(event OnComponentBeginOverlap(Box2)
  (params (OverlappedComponent :type Primitive%20Component%20Object%20Reference) (OtherActor :type Actor%20Object%20Reference) (OtherComp :type Primitive%20Component%20Object%20Reference) (OtherBodyIndex :type Integer) (bFromSweep :type Boolean) (SweepResult :type Hit%20Result%20Structure%20%28by%20ref%29))
  (if (not (Variables|/Game/Blueprint/BP_Timer.BP_Timer_C|GetRewindStateRef (Variables|Default|GetTimerRef)))
    (if (== OtherActor (Variables|Default|GetBombCoreRef))
      (Variables|/Game/Blueprint/BP_Timer.BP_Timer_C|SetTime (Variables|Default|GetTimerRef) 1.0))))

(event OnComponentBeginOverlap(Box3)
  (params (OverlappedComponent :type Primitive%20Component%20Object%20Reference) (OtherActor :type Actor%20Object%20Reference) (OtherComp :type Primitive%20Component%20Object%20Reference) (OtherBodyIndex :type Integer) (bFromSweep :type Boolean) (SweepResult :type Hit%20Result%20Structure%20%28by%20ref%29))
  (if (not (Variables|/Game/Blueprint/BP_Timer.BP_Timer_C|GetRewindStateRef (Variables|Default|GetTimerRef)))
    (if (== OtherActor (Variables|Default|GetBombCoreRef))
      (Variables|/Game/Blueprint/BP_Timer.BP_Timer_C|SetTime (Variables|Default|GetTimerRef) 1.0))))

(event EventBeginPlay
  (bind _asbp_timer (Utilities|Casting|CastToBP_TimerClass "/Game/Blueprint/BP_Timer.BP_Timer_C"))
  (bind _returnvalue (Actor|GetActorOfClass _asbp_timer))
  (Variables|Default|SetTimerRef _returnvalue)
  (bind _asbp_core_bomb (Utilities|Casting|CastToBP_CoreBombClass "/Game/Blueprint/BP_CoreBomb.BP_CoreBomb_C"))
  (bind _returnvalue_2 (Actor|GetActorOfClass _asbp_core_bomb))
  (Variables|Default|SetBombCoreRef _returnvalue_2))

(event Collision|EventActorBeginOverlap
  (params (OtherActor :type Actor%20Object%20Reference)))

(event EventTick
  (params (DeltaSeconds :type Float%20%28single-precision%29))
  (Utilities|FlowControl|Sequence
    (:then_0
      (if (<= (Variables|/Game/Blueprint/BP_Timer.BP_Timer_C|GetTime (Variables|Default|GetTimerRef)) 0.0)
        (Utilities|FlowControl|DoOnce false :!label _label
          (:Completed
            (Effects|Particles|Trails|BeginTrails (Variables|Default|GetExplosion) "None" "None" "ETrailWidthMode_FromCentre" 0.0)
            (Audio|PlaySoundatLocation "/Game/StarterContent/Audio/Explosion_Cue.Explosion_Cue" (Transformation|GetWorldLocation (Variables|Default|GetBombSkeletal)) "0, 0, 0" 1.0 1.0 0.0 0 0 0)
            (Utilities|FlowControl|Delay 3.0)
            (Effects|Particles|Trails|EndTrails (Variables|Default|GetExplosion))))
        (else
          (goto _label Reset))))
    (:then_1
      (if true
        (for _array_element (Variables|Default|GetScrewArray)
          _)))))

(fn ConstructionScript)