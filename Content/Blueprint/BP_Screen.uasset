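; BP_Screen is a screen actor that displays the time from a referenced timer as text.
; On BeginPlay, one TypeScreen option swaps the Screen to a color grid material and hides the TextRender.
; Tick copies TimerRef's Time into the TextRender every frame, regardless of screen type.
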(event EventBeginPlay
  (if (Utilities|Enum|Equal(Enum) (Variables|Default|GetTypeScreen) "NewEnumerator1")
    (Rendering|Material|SetMaterial (Variables|Default|GetScreen) 0 "/Game/StarterContent/Materials/M_ColorGrid_LowSpec.M_ColorGrid_LowSpec")
    (Rendering|SetVisibility (Variables|Default|GetTextRender) false false)))

(event Collision|EventActorBeginOverlap
  (params (OtherActor :type Actor%20Object%20Reference)))

(event EventTick
  (params (DeltaSeconds :type Float%20%28single-precision%29))
  (Rendering|Components|TextRender|SetText (Variables|Default|GetTextRender) (Utilities|Text|ToText(Float) (Variables|/Game/Blueprint/BP_Timer.BP_Timer_C|GetTime (Variables|Default|GetTimerRef)) "HalfToEven")))

(fn ConstructionScript)