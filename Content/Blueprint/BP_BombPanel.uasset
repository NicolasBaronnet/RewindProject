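; BP_BombPanel is a bomb panel that detaches under physics once all of its screws are unscrewed.
; Each tick it counts the unscrewed entries in ScrewsRef and, when all are out, enables physics simulation on its static mesh through a DoOnce.
; It also polls TimerRef each tick and switches physics off while the rewind state is set; the DoOnce is never reset here.
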(event EventBeginPlay
  (|CallParentFunction) ; This node is disabled and will not be called.\nDrag off pins to build functionality.
)

(event Collision|EventActorBeginOverlap
  (params (OtherActor :type Actor%20Object%20Reference)))

(event EventTick
  (params (DeltaSeconds :type Float%20%28single-precision%29))
  (|CallParentFunction DeltaSeconds)
  (Utilities|FlowControl|Sequence
    (:then_0
      (Variables|Default|SetCmpt 0)
      (for _array_element (Variables|Default|GetScrewsRef)
        (if (Variables|/Game/Blueprint/BP_Screw.BP_Screw_C|GetUnScrewed _array_element)
          (Math|Integer|IncrementInt (Variables|Default|GetCmpt))))
      (if (== (Utilities|Array|Length (Variables|Default|GetScrewsRef)) (Variables|Default|GetCmpt))
        (Utilities|FlowControl|DoOnce false
          (:Completed
            (Physics|SetSimulatePhysics (Variables|Default|GetStaticMesh) true)))))
    (:then_1
      (if (Variables|/Game/Blueprint/BP_Timer.BP_Timer_C|GetRewindStateRef (Variables|Default|GetTimerRef))
        (Physics|SetSimulatePhysics (Variables|Default|GetStaticMesh) false)))))

(fn ConstructionScript
  (|CallParentFunction))