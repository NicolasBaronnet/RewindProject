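; BP_PhonePanel is an actor whose panel component attaches to a referenced phone and rotates when a button is activated.
; On BeginPlay it binds each entry in BPButton to ReturnPanel and snaps the panel to the phone's root.
; ReturnPanel starts rotation if the BeginPlay loop's current element has the first button type.
; Tick pitches the panel at a frame-rate-independent speed until its world pitch drops below zero.
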(event Custom|Return%20Panel
  (if (Utilities|Enum|Equal(Enum) (Variables|/Game/Blueprint/BP_ButtonBase.BP_ButtonBase_C|GetTypeBouton (stale EventBeginPlay _array_element)) "NewEnumerator0")
    (Variables|Default|SetRotate true)))

(event EventBeginPlay
  (for _array_element (Variables|Default|GetBP_Button)
    (EventDispatchers|BindEventtoButtonActivated _array_element (delegate Custom|Return%20Panel))
    (Transformation|AttachComponentToComponent (Variables|Default|GetPanel) (Variables|/Script/Engine.Actor|GetRootComponent (Variables|Default|GetPhoneRef)) "None" "SnapToTarget" "SnapToTarget" "KeepWorld" true)))

(event Collision|EventActorBeginOverlap
  (params (OtherActor :type Actor%20Object%20Reference)))

(event EventTick
  (params (DeltaSeconds :type Float%20%28single-precision%29))
  (bind _panel (Variables|Default|GetPanel))
  (if (Variables|Default|GetRotate)
    (Transformation|AddLocalRotation _panel (* (Math|Rotator|MakeRotator 0.0 (Variables|Default|GetRoationSpeed) 0.0) DeltaSeconds) false false)
    (if (< (.pitch (Transformation|GetWorldRotation _panel)) 0.0)
      (Variables|Default|SetRotate false))))

(fn ConstructionScript)