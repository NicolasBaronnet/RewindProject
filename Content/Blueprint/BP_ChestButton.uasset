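; BP_ChestButton is a grabbable button actor, by its name for a chest, that rotates in place when picked up.
; BeginPlay caches the static mesh's starting world transform.
; Pickup is a one-shot update that keeps the original location and scale and copies only the roll of the grabbing component, leaving pitch and yaw unconnected.
; Drop does nothing, and the grab queries return a "None" socket and a fixed grab behavior.
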(event EventBeginPlay
  (|CallParentFunction)
  (Variables|Default|SetStartTransform (Transformation|GetWorldTransform (Variables|Default|GetStaticMesh))))

(event Collision|EventActorBeginOverlap
  (params (OtherActor :type Actor%20Object%20Reference)))

(event EventDrop)

(event EventTick
  (params (DeltaSeconds :type Float%20%28single-precision%29))
  (|CallParentFunction DeltaSeconds) ; This node is disabled and will not be called.\nDrag off pins to build functionality.
)

(event EventPickup
  (params (AttachTo :type Scene%20Component%20Object%20Reference))
  (bind _starttransform (Variables|Default|GetStartTransform))
  (bind (_location _rotation _scale) (Math|Transform|BreakTransform _starttransform))
  (Transformation|SetWorldTransform (Variables|Default|GetStaticMesh) (Math|Transform|MakeTransform _location (Math|Rotator|MakeRotator (.roll (.rotation (Transformation|GetWorldTransform AttachTo))) 0.0 0.0) _scale) false false))

(fn ConstructionScript
  (|CallParentFunction))

(fn GetSocketName
  (return "None"))

(fn GrabBehvior
  (return "NewEnumerator0"))