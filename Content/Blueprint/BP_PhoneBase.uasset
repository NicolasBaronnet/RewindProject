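; VR phone base with a ten-digit keypad that the player presses with motion controller hands.
; On BeginPlay it pauses the ring sound and caches the pawn's two controllers as valid pressers.
; Each button overlap, debounced by DoOnce, runs ButtonFunction, which beeps and appends the digit, restarting after four.
; A full code fetches BP_Phone's code, but the comparison that prints success is disconnected.
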(event OnComponentBeginOverlap(Bouton1)
  (params (OverlappedComponent :type Primitive%20Component%20Object%20Reference) (OtherActor :type Actor%20Object%20Reference) (OtherComp :type Primitive%20Component%20Object%20Reference) (OtherBodyIndex :type Integer) (bFromSweep :type Boolean) (SweepResult :type Hit%20Result%20Structure%20%28by%20ref%29))
  ;[1 1 1] Clavier du téléphone
  (Utilities|FlowControl|DoOnce false
    (:Completed
      (bind _output_get (Variables|Default|SetButtonNumber 1))
      (CallFunction|ButtonFunction OtherActor _output_get)
      ;[1 1 1] Vérification du code
      (if (== (Utilities|Array|Length (Variables|Default|GetCode)) 4)
        (bind _returnvalue (Actor|GetActorOfClass "/Game/Blueprint/BP_Phone.BP_Phone_C"))
        (Variables|Default|SetTrueCode (Variables|/Game/Blueprint/BP_Phone.BP_Phone_C|GetCode _returnvalue))))))

(event OnComponentEndOverlap(Bouton1)
  (params (OverlappedComponent :type Primitive%20Component%20Object%20Reference) (OtherActor :type Actor%20Object%20Reference) (OtherComp :type Primitive%20Component%20Object%20Reference) (OtherBodyIndex :type Integer))
  ;[1 1 1] Clavier du téléphone
  (Variables|Default|SetGoodCollision false)
  (Utilities|FlowControl|Delay 0.5)
  (Utilities|FlowControl|DoOnce false) ; enters at Reset
)

(event OnComponentBeginOverlap(Bouton6)
  (params (OverlappedComponent :type Primitive%20Component%20Object%20Reference) (OtherActor :type Actor%20Object%20Reference) (OtherComp :type Primitive%20Component%20Object%20Reference) (OtherBodyIndex :type Integer) (bFromSweep :type Boolean) (SweepResult :type Hit%20Result%20Structure%20%28by%20ref%29))
  ;[1 1 1] Clavier du téléphone
  (Utilities|FlowControl|DoOnce false
    (:Completed
      (bind _output_get (Variables|Default|SetButtonNumber 6))
      (CallFunction|ButtonFunction OtherActor _output_get)
      ;[1 1 1] Vérification du code
      (if (== (Utilities|Array|Length (Variables|Default|GetCode)) 4)
        (bind _returnvalue (Actor|GetActorOfClass "/Game/Blueprint/BP_Phone.BP_Phone_C"))
        (Variables|Default|SetTrueCode (Variables|/Game/Blueprint/BP_Phone.BP_Phone_C|GetCode _returnvalue))))))

(event OnComponentEndOverlap(Bouton6)
  (params (OverlappedComponent :type Primitive%20Component%20Object%20Reference) (OtherActor :type Actor%20Object%20Reference) (OtherComp :type Primitive%20Component%20Object%20Reference) (OtherBodyIndex :type Integer))
  ;[1 1 1] Clavier du téléphone
  (Variables|Default|SetGoodCollision false)
  (Utilities|FlowControl|Delay 0.5)
  (Utilities|FlowControl|DoOnce false) ; enters at Reset
)

(event OnComponentBeginOverlap(Bouton2)
  (params (OverlappedComponent :type Primitive%20Component%20Object%20Reference) (OtherActor :type Actor%20Object%20Reference) (OtherComp :type Primitive%20Component%20Object%20Reference) (OtherBodyIndex :type Integer) (bFromSweep :type Boolean) (SweepResult :type Hit%20Result%20Structure%20%28by%20ref%29))
  ;[1 1 1] Clavier du téléphone
  (Utilities|FlowControl|DoOnce false
    (:Completed
      (bind _output_get (Variables|Default|SetButtonNumber 2))
      (CallFunction|ButtonFunction OtherActor _output_get)
      ;[1 1 1] Vérification du code
      (if (== (Utilities|Array|Length (Variables|Default|GetCode)) 4)
        (bind _returnvalue (Actor|GetActorOfClass "/Game/Blueprint/BP_Phone.BP_Phone_C"))
        (Variables|Default|SetTrueCode (Variables|/Game/Blueprint/BP_Phone.BP_Phone_C|GetCode _returnvalue))))))

(event OnComponentEndOverlap(Bouton2)
  (params (OverlappedComponent :type Primitive%20Component%20Object%20Reference) (OtherActor :type Actor%20Object%20Reference) (OtherComp :type Primitive%20Component%20Object%20Reference) (OtherBodyIndex :type Integer))
  ;[1 1 1] Clavier du téléphone
  (Variables|Default|SetGoodCollision false)
  (Utilities|FlowControl|Delay 0.5)
  (Utilities|FlowControl|DoOnce false) ; enters at Reset
)

(event OnComponentBeginOverlap(Bouton0)
  (params (OverlappedComponent :type Primitive%20Component%20Object%20Reference) (OtherActor :type Actor%20Object%20Reference) (OtherComp :type Primitive%20Component%20Object%20Reference) (OtherBodyIndex :type Integer) (bFromSweep :type Boolean) (SweepResult :type Hit%20Result%20Structure%20%28by%20ref%29))
  ;[1 1 1] Clavier du téléphone
  (Utilities|FlowControl|DoOnce false
    (:Completed
      (Variables|Default|SetButtonNumber 0)
      (CallFunction|ButtonFunction OtherActor)
      ;[1 1 1] Vérification du code
      (if (== (Utilities|Array|Length (Variables|Default|GetCode)) 4)
        (bind _returnvalue (Actor|GetActorOfClass "/Game/Blueprint/BP_Phone.BP_Phone_C"))
        (Variables|Default|SetTrueCode (Variables|/Game/Blueprint/BP_Phone.BP_Phone_C|GetCode _returnvalue))))))

(event OnComponentEndOverlap(Bouton0)
  (params (OverlappedComponent :type Primitive%20Component%20Object%20Reference) (OtherActor :type Actor%20Object%20Reference) (OtherComp :type Primitive%20Component%20Object%20Reference) (OtherBodyIndex :type Integer))
  ;[1 1 1] Clavier du téléphone
  (Variables|Default|SetGoodCollision false)
  (Utilities|FlowControl|Delay 0.5)
  (Utilities|FlowControl|DoOnce false) ; enters at Reset
)

(event OnComponentBeginOverlap(Bouton7)
  (params (OverlappedComponent :type Primitive%20Component%20Object%20Reference) (OtherActor :type Actor%20Object%20Reference) (OtherComp :type Primitive%20Component%20Object%20Reference) (OtherBodyIndex :type Integer) (bFromSweep :type Boolean) (SweepResult :type Hit%20Result%20Structure%20%28by%20ref%29))
  ;[1 1 1] Clavier du téléphone
  (Utilities|FlowControl|DoOnce false
    (:Completed
      (bind _output_get (Variables|Default|SetButtonNumber 7))
      (CallFunction|ButtonFunction OtherActor _output_get)
      ;[1 1 1] Vérification du code
      (if (== (Utilities|Array|Length (Variables|Default|GetCode)) 4)
        (bind _returnvalue (Actor|GetActorOfClass "/Game/Blueprint/BP_Phone.BP_Phone_C"))
        (Variables|Default|SetTrueCode (Variables|/Game/Blueprint/BP_Phone.BP_Phone_C|GetCode _returnvalue))))))

(event OnComponentEndOverlap(Bouton7)
  (params (OverlappedComponent :type Primitive%20Component%20Object%20Reference) (OtherActor :type Actor%20Object%20Reference) (OtherComp :type Primitive%20Component%20Object%20Reference) (OtherBodyIndex :type Integer))
  ;[1 1 1] Clavier du téléphone
  (Variables|Default|SetGoodCollision false)
  (Utilities|FlowControl|Delay 0.5)
  (Utilities|FlowControl|DoOnce false) ; enters at Reset
)

(event OnComponentBeginOverlap(Bouton8)
  (params (OverlappedComponent :type Primitive%20Component%20Object%20Reference) (OtherActor :type Actor%20Object%20Reference) (OtherComp :type Primitive%20Component%20Object%20Reference) (OtherBodyIndex :type Integer) (bFromSweep :type Boolean) (SweepResult :type Hit%20Result%20Structure%20%28by%20ref%29))
  ;[1 1 1] Clavier du téléphone
  (Utilities|FlowControl|DoOnce false
    (:Completed
      (bind _output_get (Variables|Default|SetButtonNumber 8))
      (CallFunction|ButtonFunction OtherActor _output_get)
      ;[1 1 1] Vérification du code
      (if (== (Utilities|Array|Length (Variables|Default|GetCode)) 4)
        (bind _returnvalue (Actor|GetActorOfClass "/Game/Blueprint/BP_Phone.BP_Phone_C"))
        (Variables|Default|SetTrueCode (Variables|/Game/Blueprint/BP_Phone.BP_Phone_C|GetCode _returnvalue))))))

(event OnComponentEndOverlap(Bouton8)
  (params (OverlappedComponent :type Primitive%20Component%20Object%20Reference) (OtherActor :type Actor%20Object%20Reference) (OtherComp :type Primitive%20Component%20Object%20Reference) (OtherBodyIndex :type Integer))
  ;[1 1 1] Clavier du téléphone
  (Variables|Default|SetGoodCollision false)
  (Utilities|FlowControl|Delay 0.5)
  (Utilities|FlowControl|DoOnce false) ; enters at Reset
)

(event OnComponentBeginOverlap(Bouton3)
  (params (OverlappedComponent :type Primitive%20Component%20Object%20Reference) (OtherActor :type Actor%20Object%20Reference) (OtherComp :type Primitive%20Component%20Object%20Reference) (OtherBodyIndex :type Integer) (bFromSweep :type Boolean) (SweepResult :type Hit%20Result%20Structure%20%28by%20ref%29))
  ;[1 1 1] Clavier du téléphone
  (Utilities|FlowControl|DoOnce false
    (:Completed
      (bind _output_get (Variables|Default|SetButtonNumber 3))
      (CallFunction|ButtonFunction OtherActor _output_get)
      ;[1 1 1] Vérification du code
      (if (== (Utilities|Array|Length (Variables|Default|GetCode)) 4)
        (bind _returnvalue (Actor|GetActorOfClass "/Game/Blueprint/BP_Phone.BP_Phone_C"))
        (Variables|Default|SetTrueCode (Variables|/Game/Blueprint/BP_Phone.BP_Phone_C|GetCode _returnvalue))))))

(event OnComponentBeginOverlap(Bouton9)
  (params (OverlappedComponent :type Primitive%20Component%20Object%20Reference) (OtherActor :type Actor%20Object%20Reference) (OtherComp :type Primitive%20Component%20Object%20Reference) (OtherBodyIndex :type Integer) (bFromSweep :type Boolean) (SweepResult :type Hit%20Result%20Structure%20%28by%20ref%29))
  ;[1 1 1] Clavier du téléphone
  (Utilities|FlowControl|DoOnce false
    (:Completed
      (bind _output_get (Variables|Default|SetButtonNumber 9))
      (CallFunction|ButtonFunction OtherActor _output_get)
      ;[1 1 1] Vérification du code
      (if (== (Utilities|Array|Length (Variables|Default|GetCode)) 4)
        (bind _returnvalue (Actor|GetActorOfClass "/Game/Blueprint/BP_Phone.BP_Phone_C"))
        (Variables|Default|SetTrueCode (Variables|/Game/Blueprint/BP_Phone.BP_Phone_C|GetCode _returnvalue))))))

(event OnComponentEndOverlap(Bouton9)
  (params (OverlappedComponent :type Primitive%20Component%20Object%20Reference) (OtherActor :type Actor%20Object%20Reference) (OtherComp :type Primitive%20Component%20Object%20Reference) (OtherBodyIndex :type Integer))
  ;[1 1 1] Clavier du téléphone
  (Variables|Default|SetGoodCollision false)
  (Utilities|FlowControl|Delay 0.5)
  (Utilities|FlowControl|DoOnce false) ; enters at Reset
)

(event OnComponentEndOverlap(Bouton3)
  (params (OverlappedComponent :type Primitive%20Component%20Object%20Reference) (OtherActor :type Actor%20Object%20Reference) (OtherComp :type Primitive%20Component%20Object%20Reference) (OtherBodyIndex :type Integer))
  ;[1 1 1] Clavier du téléphone
  (Variables|Default|SetGoodCollision false)
  (Utilities|FlowControl|Delay 0.5)
  (Utilities|FlowControl|DoOnce false) ; enters at Reset
)

(event OnComponentBeginOverlap(Bouton4)
  (params (OverlappedComponent :type Primitive%20Component%20Object%20Reference) (OtherActor :type Actor%20Object%20Reference) (OtherComp :type Primitive%20Component%20Object%20Reference) (OtherBodyIndex :type Integer) (bFromSweep :type Boolean) (SweepResult :type Hit%20Result%20Structure%20%28by%20ref%29))
  ;[1 1 1] Clavier du téléphone
  (Utilities|FlowControl|DoOnce false
    (:Completed
      (bind _output_get (Variables|Default|SetButtonNumber 4))
      (CallFunction|ButtonFunction OtherActor _output_get)
      ;[1 1 1] Vérification du code
      (if (== (Utilities|Array|Length (Variables|Default|GetCode)) 4)
        (bind _returnvalue (Actor|GetActorOfClass "/Game/Blueprint/BP_Phone.BP_Phone_C"))
        (Variables|Default|SetTrueCode (Variables|/Game/Blueprint/BP_Phone.BP_Phone_C|GetCode _returnvalue))))))

(event OnComponentEndOverlap(Bouton4)
  (params (OverlappedComponent :type Primitive%20Component%20Object%20Reference) (OtherActor :type Actor%20Object%20Reference) (OtherComp :type Primitive%20Component%20Object%20Reference) (OtherBodyIndex :type Integer))
  ;[1 1 1] Clavier du téléphone
  (Variables|Default|SetGoodCollision false)
  (Utilities|FlowControl|Delay 0.5)
  (Utilities|FlowControl|DoOnce false) ; enters at Reset
)

(event OnComponentBeginOverlap(Bouton5)
  (params (OverlappedComponent :type Primitive%20Component%20Object%20Reference) (OtherActor :type Actor%20Object%20Reference) (OtherComp :type Primitive%20Component%20Object%20Reference) (OtherBodyIndex :type Integer) (bFromSweep :type Boolean) (SweepResult :type Hit%20Result%20Structure%20%28by%20ref%29))
  ;[1 1 1] Clavier du téléphone
  (Utilities|FlowControl|DoOnce false
    (:Completed
      (bind _output_get (Variables|Default|SetButtonNumber 5))
      (CallFunction|ButtonFunction OtherActor _output_get)
      ;[1 1 1] Vérification du code
      (if (== (Utilities|Array|Length (Variables|Default|GetCode)) 4)
        (bind _returnvalue (Actor|GetActorOfClass "/Game/Blueprint/BP_Phone.BP_Phone_C"))
        (Variables|Default|SetTrueCode (Variables|/Game/Blueprint/BP_Phone.BP_Phone_C|GetCode _returnvalue))))))

(event OnComponentEndOverlap(Bouton5)
  (params (OverlappedComponent :type Primitive%20Component%20Object%20Reference) (OtherActor :type Actor%20Object%20Reference) (OtherComp :type Primitive%20Component%20Object%20Reference) (OtherBodyIndex :type Integer))
  ;[1 1 1] Clavier du téléphone
  (Variables|Default|SetGoodCollision false)
  (Utilities|FlowControl|Delay 0.5)
  (Utilities|FlowControl|DoOnce false) ; enters at Reset
)

(event EventBeginPlay
  (Utilities|FlowControl|Delay 0.2)
  (Class|AudioComponent|SetPaused (Variables|Default|GetSC_PhoneRing) true)
  (bind _returnvalue (Actor|GetActorOfClass "/Game/Blueprint/MotionControllerPawn.MotionControllerPawn_C"))
  (Utilities|IsValid (Variables|/Game/Blueprint/MotionControllerPawn.MotionControllerPawn_C|GetLeftController _returnvalue)
    (:Is%20Valid
      (Utilities|Array|Add (Variables|Default|GetHandCollisions) (Variables|/Game/Blueprint/MotionControllerPawn.MotionControllerPawn_C|GetLeftController _returnvalue))
      (Utilities|Array|Add (Variables|Default|GetHandCollisions) (Variables|/Game/Blueprint/MotionControllerPawn.MotionControllerPawn_C|GetRightController _returnvalue)))))

(event Collision|EventActorBeginOverlap
  (params (OtherActor :type Actor%20Object%20Reference)))

(event EventTick
  (params (DeltaSeconds :type Float%20%28single-precision%29)))

(fn ConstructionScript)

(fn ButtonFunction
  (params (A :type Object%20Object%20Reference) (ButtonNumber :type Integer))
  (for _array_element (Variables|Default|GetHandCollisions)
    (if (== A _array_element)
      (Variables|Default|SetGoodCollision true)))
  (if (Variables|Default|GetGoodCollision)
    (Audio|PlaySound2D "/Game/Sounds/Ambiant/BipPhone.BipPhone" 1.0 1.0 0.0 0 0)
    (if (> (Utilities|Array|Length (Variables|Default|GetCode)) 3)
      (Utilities|Array|Clear (Variables|Default|GetCode))
      (Utilities|Array|Add (Variables|Default|GetCode) (Math|Integer|Absolute(Integer) ButtonNumber))
      (return false)
      (else
        (Utilities|Array|Add (Variables|Default|GetCode) (Math|Integer|Absolute(Integer) ButtonNumber))))))

(fn GetSocketName
  (return "None"))

(fn GrabBehvior
  (return "NewEnumerator0"))