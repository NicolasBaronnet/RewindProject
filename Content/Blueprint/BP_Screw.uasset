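; BP_Screw is a screw actor that turns when a BP_ScrewDriver is rotated inside its box trigger.
; Overlap with the screwdriver's Collision component stores a reference and starting rotation in box space; ending the overlap clears the reference.
; Tick compares world yaw with the last sample, turning the mesh only as yaw decreases, with each step clamped to ten degrees.
; Debug prints trace interaction and rotation deltas.
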(event OnComponentBeginOverlap(Box)
  (params (OverlappedComponent :type Primitive%20Component%20Object%20Reference) (OtherActor :type Actor%20Object%20Reference) (OtherComp :type Primitive%20Component%20Object%20Reference) (OtherBodyIndex :type Integer) (bFromSweep :type Boolean) (SweepResult :type Hit%20Result%20Structure%20%28by%20ref%29))
  (bind _asbp_screw_driver (Utilities|Casting|CastToBP_ScrewDriver OtherActor))
  (if (== OtherComp (Variables|/Game/Blueprint/BP_ScrewDriver.BP_ScrewDriver_C|GetCollision _asbp_screw_driver))
    (CallFunction|StartInteract _asbp_screw_driver)))

(event OnComponentEndOverlap(Box)
  (params (OverlappedComponent :type Primitive%20Component%20Object%20Reference) (OtherActor :type Actor%20Object%20Reference) (OtherComp :type Primitive%20Component%20Object%20Reference) (OtherBodyIndex :type Integer))
  (bind _bpscrewdriverref (Variables|Default|GetBPScrewDriverRef))
  (Utilities|IsValid _bpscrewdriverref
    (:Is%20Valid
      (if (and (== OtherActor _bpscrewdriverref) (== OtherComp (Variables|/Game/Blueprint/BP_ScrewDriver.BP_ScrewDriver_C|GetCollision _bpscrewdriverref)))
        (CallFunction|StopInteract)))))

(event Custom|StartInteract
  (params (ScrewDriver :type BP%20Screw%20Driver%20Object%20Reference))
  (Variables|Default|SetLastRotation (Math|Transform|InverseTransformRotation (Transformation|GetWorldTransform (Variables|Default|GetBox)) (Transformation|GetWorldRotation (Variables|/Game/Blueprint/BP_RewindableObject.BP_RewindableObject_C|GetDefaultSceneRoot ScrewDriver))))
  (Variables|Default|SetBPScrewDriverRef ScrewDriver)
  (Development|PrintString "starting interaction"))

(event Custom|StopInteract
  (Variables|Default|SetBPScrewDriverRef 0)
  (Development|PrintString "stopping interaction"))

(event EventBeginPlay)

(event Collision|EventActorBeginOverlap
  (params (OtherActor :type Actor%20Object%20Reference)))

(event EventTick
  (params (DeltaSeconds :type Float%20%28single-precision%29))
  (Utilities|IsValid (Variables|Default|GetBPScrewDriverRef)
    (:Is%20Valid
      (bind _output_get (Variables|Default|SetCurrentRotation (Transformation|GetWorldRotation (Variables|/Game/Blueprint/BP_RewindableObject.BP_RewindableObject_C|GetDefaultSceneRoot (Variables|Default|GetBPScrewDriverRef)))))
      (if (> (- (.yaw (Variables|Default|GetLastRotation)) (.Yaw (Math|Rotator|BreakRotator _output_get))) 0.0)
        (Development|PrintString (Utilities|String|Append (Utilities|String|ToString(Float) (.yaw (Variables|Default|GetLastRotation))) " - " (Utilities|String|ToString(Float) (.Yaw (Math|Rotator|BreakRotator _output_get))) " = " (Utilities|String|ToString(Float) (- (.yaw (Variables|Default|GetLastRotation)) (.Yaw (Math|Rotator|BreakRotator _output_get))))))
        (Transformation|AddRelativeRotation (Variables|Default|GetStaticMesh) (Math|Rotator|MakeRotator 0.0 0.0 (Math|Float|ClampAngle (- (.yaw (Variables|Default|GetLastRotation)) (.Yaw (Math|Rotator|BreakRotator _output_get))) 0.0 1e+01)) false false)
        (Variables|Default|SetLastRotation _output_get)
        (else
          (Variables|Default|SetLastRotation _output_get))))))

(fn ConstructionScript)