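; VR phone that speaks a randomized four-sound code when picked up while ringing.
; Grabbing within its sphere shuffles CodeArray and, if BP_PhoneBase is ringing, fires a DoOnce that Tick re-arms while BP_Timer is at zero or below.
; It stops the ring, plays four sounds with delays, then fills and debug-prints Code with matching BaseArray indices, in base order.
; GetSocketName picks the left or right hand socket.
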(event OnComponentBeginOverlap(Sphere)
  (params (OverlappedComponent :type Primitive%20Component%20Object%20Reference) (OtherActor :type Actor%20Object%20Reference) (OtherComp :type Primitive%20Component%20Object%20Reference) (OtherBodyIndex :type Integer) (bFromSweep :type Boolean) (SweepResult :type Hit%20Result%20Structure%20%28by%20ref%29))
  (bind _asmotion_controller_pawn (Utilities|Casting|CastToMotionControllerPawn (Game|Player|GetPlayerPawn 0)))
  (if (or (Variables|/Game/Blueprint/MotionControllerPawn.MotionControllerPawn_C|GetGrabLeft _asmotion_controller_pawn) (Variables|/Game/Blueprint/MotionControllerPawn.MotionControllerPawn_C|GetGrabRight _asmotion_controller_pawn))
    (Utilities|Array|Shuffle (Variables|Default|GetCodeArray))
    (bind _asbp_phone_base (Utilities|Casting|CastToBP_PhoneBaseClass "/Game/Blueprint/BP_PhoneBase.BP_PhoneBase_C"))
    (bind _returnvalue (Actor|GetActorOfClass _asbp_phone_base))
    (if (Components|Activation|IsActive (Variables|/Game/Blueprint/BP_PhoneBase.BP_PhoneBase_C|GetSC_PhoneRing _returnvalue))
      (Utilities|FlowControl|DoOnce false
        (:Completed
          (Audio|Components|Audio|Stop (Variables|/Game/Blueprint/BP_PhoneBase.BP_PhoneBase_C|GetSC_PhoneRing _returnvalue))
          (Audio|Components|Audio|Play (Utilities|Array|Get(acopy) (Variables|Default|GetCodeArray)) 0.0)
          (Utilities|FlowControl|Delay 1.0)
          (Audio|Components|Audio|Play (Utilities|Array|Get(acopy) (Variables|Default|GetCodeArray) 1) 0.0)
          (Utilities|FlowControl|Delay 1.0)
          (Audio|Components|Audio|Play (Utilities|Array|Get(acopy) (Variables|Default|GetCodeArray) 2) 1.5)
          (Utilities|FlowControl|Delay 1.0)
          (Audio|Components|Audio|Play (Utilities|Array|Get(acopy) (Variables|Default|GetCodeArray) 3) 0.0)
          (Utilities|FlowControl|Delay 3.0)
          (for (_array_element _array_index) (Variables|Default|GetBaseArray)
            (bind _output_get (Variables|Default|SetActiveSound _array_element))
            (for _array_element_2 (Variables|Default|GetCodeArray)
              (if (== _array_element_2 _output_get)
                (Utilities|Array|Add (Variables|Default|GetCode) _array_index))))
          ;[1 1 1] Debug
          (for _array_element_3 (Variables|Default|GetCode)
            (Development|PrintString (Utilities|String|ToString(Integer) _array_element_3))))))))

(event EventBeginPlay
  (bind _4 (Variables|Default|Get4))
  (bind _3 (Variables|Default|Get3))
  (bind _2 (Variables|Default|Get2))
  (bind _1 (Variables|Default|Get1))
  (bind _0 (Variables|Default|Get0))
  (bind _8 (Variables|Default|Get8))
  (bind _7 (Variables|Default|Get7))
  (bind _6 (Variables|Default|Get6))
  (bind _5 (Variables|Default|Get5))
  (bind _9 (Variables|Default|Get9))
  (bind _array (Utilities|Array|MakeArray _0 _1 _2 _3 _4 _5 _6 _7 _8 _9))
  (|CallParentFunction)
  (Variables|Default|SetCodeArray _array)
  (Variables|Default|SetBaseArray _array))

(event Collision|EventActorBeginOverlap
  (params (OtherActor :type Actor%20Object%20Reference))
  (|CallParentFunction OtherActor))

(event EventTick
  (params (DeltaSeconds :type Float%20%28single-precision%29))
  (|CallParentFunction DeltaSeconds)
  (bind _asbp_timer (Utilities|Casting|CastToBP_TimerClass))
  (bind _returnvalue (Actor|GetActorOfClass _asbp_timer))
  (if (<= (Variables|/Game/Blueprint/BP_Timer.BP_Timer_C|GetTime _returnvalue) 0.0)
    (Utilities|FlowControl|DoOnce false) ; enters at Reset
  ))

(fn ConstructionScript
  (|CallParentFunction))

(fn GetSocketName
  (bind _asmotion_controller_pawn (Utilities|Casting|CastToMotionControllerPawn (Game|Player|GetPlayerPawn 0)))
  (if (Variables|/Game/Blueprint/MotionControllerPawn.MotionControllerPawn_C|GetGrabLeft _asmotion_controller_pawn)
    (LocalVariables|SetSocketName (Utilities|String|StringToName (Utilities|String|Append "TakePhone" "_L")))
    (else
      (LocalVariables|SetSocketName (Utilities|String|StringToName (Utilities|String|Append "TakePhone" "_R")))))
  (return (LocalVariables|GetSocketName)))