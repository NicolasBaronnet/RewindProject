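; Game timer Blueprint that keeps a Time value, stepped each second up or down according to the player's RewindState.
; Tick sets looping timers for each direction, whose events pause the opposite one, and applies pending time additions.
; At zero it disables input until all BP_RewindableObject histories are nearly empty, then adds time.
; Falling below thresholds fires DoOnce events, re-armed at zero: phone ringing, plus print-only smoke and darkness placeholders.
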(event Custom|TimeDown
  ;[1 1 1] Gestion Timer
  (CallFunction|DecrementTime (Variables|Default|GetForwardTimer) (Variables|Default|GetBackwardTimer)))

(event Custom|TimeUp
  ;[1 1 1] Gestion Timer
  (CallFunction|IncrementTime (Variables|Default|GetBackwardTimer) (Variables|Default|GetForwardTimer))
  (Utilities|FlowControl|DoOnce false
    (:Completed
      (Utilities|Time|ClearandInvalidateTimerbyHandle (stale EventBeginPlay _returnvalue)))))

(event EventBeginPlay
  (bind _returnvalue (Utilities|Time|SetTimerbyEvent (delegate Custom|TimeDown) 1.0 true)))

(event EventTick
  (params (DeltaSeconds :type Float%20%28single-precision%29))
  (Utilities|FlowControl|Sequence
    (:then_0
      ;[1 1 1] Gestion Timer
      (bind _asmotion_controller_pawn (Utilities|Casting|CastToMotionControllerPawn (Game|Player|GetPlayerPawn 0)))
      (bind _output_get (Variables|Default|SetRewindStateRef (Variables|/Game/Blueprint/MotionControllerPawn.MotionControllerPawn_C|GetRewindState _asmotion_controller_pawn)))
      (if _output_get
        (bind _returnvalue (Utilities|Time|SetTimerbyEvent (delegate Custom|TimeDown) 1.0 true))
        (Variables|Default|SetBackwardTimer _returnvalue)
        (elif (!= (Variables|Default|GetTime) 0.0)
          (bind _returnvalue_2 (Utilities|Time|SetTimerbyEvent (delegate Custom|TimeUp) 1.0 true))
          (Variables|Default|SetForwardTimer _returnvalue_2))))
    (:then_1
      ;[1 1 1] Enable Rewind Disable/Enable Input
      (if (== (Variables|Default|GetTime) 0.0)
        (Input|DisableInput (Game|Player|GetPlayerPawn 0) (Game|GetPlayerController 0))
        (bind _outactors (Actor|GetAllActorsOfClass "/Game/Blueprint/BP_RewindableObject.BP_RewindableObject_C"))
        (Variables|Default|SetStopRewind true)
        (for _array_element _outactors
          (if (>= (Utilities|Array|Length (Variables|/Game/Blueprint/BP_RewindableObject.BP_RewindableObject_C|GetTransformArray _array_element)) 2)
            (Variables|Default|SetStopRewind false)))
        (if (Variables|Default|GetStopRewind)
          (Variables|Default|SetTime (+ (Variables|Default|GetTime) 3e+01))
          (Input|EnableInput (Game|Player|GetPlayerPawn 0) (Game|GetPlayerController 0)))))
    (:then_2
      ;[1 1 1] Add Time Event
      (if (not (Variables|Default|GetIsAdded))
        (bind _addedtime (CallFunction|AddTime (Variables|Default|GetTimeToAdd)))
        (Variables|Default|SetTime _addedtime)
        (Variables|Default|SetIsAdded true)))
    (:then_3
      (if (<= (Variables|Default|GetTime) 0.0)
        (Utilities|FlowControl|Sequence
          (:then_0
            (goto _label Reset))
          (:then_1
            (goto _label_2 Reset))
          (:then_2
            (goto _label_3 Reset))
          (:then_3
            (Utilities|FlowControl|DoOnce false) ; enters at Reset
          ))
        (else
          (Utilities|FlowControl|Sequence
            (:then_0
              (if (< (Variables|Default|GetTime) (Variables|Default|GetTimePhoneRinging))
                (Utilities|FlowControl|DoOnce false :!label _label
                  (:Completed
                    (Variables|Default|SetIsAdded false)
                    (bind _asbp_phone_base (Utilities|Casting|CastToBP_PhoneBaseClass "/Game/Blueprint/BP_PhoneBase.BP_PhoneBase_C"))
                    (bind _returnvalue_3 (Actor|GetActorOfClass _asbp_phone_base))
                    (Class|AudioComponent|SetPaused (Variables|/Game/Blueprint/BP_PhoneBase.BP_PhoneBase_C|GetSC_PhoneRing _returnvalue_3) false)
                    (if (Variables|Default|GetPhoneCodeTrue)
                      (Variables|Default|SetTimeToAdd 15.0)
                      (Class|AudioComponent|SetPaused (Variables|/Game/Blueprint/BP_PhoneBase.BP_PhoneBase_C|GetSC_PhoneRing _returnvalue_3) false))))))
            (:then_1
              (if (< (Variables|Default|GetTime) (Variables|Default|GetTimeSmokeAppear))
                (Utilities|FlowControl|DoOnce false :!label _label_2
                  (:Completed
                    (Variables|Default|SetIsAdded false)
                    (Development|PrintString "Y fait Fumée")))))
            (:then_2
              (if (< (Variables|Default|GetTime) (Variables|Default|GetTimeLightShutdown))
                (Utilities|FlowControl|DoOnce false :!label _label_3
                  (:Completed
                    (Variables|Default|SetIsAdded false)
                    (Development|PrintString "Y fait noir")))))))))))

(fn ConstructionScript)

(fn IncrementTime
  (params (PauseEntry :type Timer%20Handle%20Structure) (PlayEntry :type Timer%20Handle%20Structure))
  (Math|Float|IncrementFloat (Variables|Default|GetTime)
    (:%20%20
      (Utilities|Time|PauseTimerbyHandle PauseEntry)
      (Utilities|Time|UnpauseTimerbyHandle PlayEntry))))

(fn DecrementTime
  (params (PauseEntry :type Timer%20Handle%20Structure) (PlayEntry :type Timer%20Handle%20Structure))
  (Math|Float|DecrementFloat (Variables|Default|GetTime)
    (:%20%20
      (Utilities|Time|PauseTimerbyHandle PauseEntry)
      (Utilities|Time|UnpauseTimerbyHandle PlayEntry))))

(fn AddTime
  (params (TimeToAdd :type Float%20%28single-precision%29))
  (bind _output_get (Variables|Default|SetTime (+ TimeToAdd (Variables|Default|GetTime))))
  (return _output_get))