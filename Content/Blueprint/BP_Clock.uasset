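; BP_Clock is a clock actor whose Small and Big meshes rotate every tick by SpeedTick.
; TimerRef's rewind state switches the Big part to a faster spin in the opposite direction, while Small is unchanged.
; The first tick spawns a clock sound at the Base after a short delay.
; RefBomb's winning event, bound on BeginPlay, stops that sound and zeroes SpeedTick once, freezing the clock.
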(event Custom|WinningLane
  (Utilities|FlowControl|DoOnce false
    (:Completed
      (Utilities|IsValid (stale EventTick _returnvalue)
        (:Is%20Valid
          (Audio|Components|Audio|Stop (stale EventTick _returnvalue)))
        (:Is%20Not%20Valid
          _))
      (Variables|Default|SetSpeedTick 0.0))))

(event EventBeginPlay
  (EventDispatchers|BindEventtoWinningEvent (Variables|Default|GetRefBomb) (delegate Custom|WinningLane)))

(event Collision|EventActorBeginOverlap
  (params (OtherActor :type Actor%20Object%20Reference)))

(event EventTick
  (params (DeltaSeconds :type Float%20%28single-precision%29))
  (bind _speedtick (Variables|Default|GetSpeedTick))
  (bind _speedtick_2 (Variables|Default|GetSpeedTick))
  (Utilities|FlowControl|Sequence
    (:then_0
      (if (Variables|/Game/Blueprint/BP_Timer.BP_Timer_C|GetRewindStateRef (Variables|Default|GetTimerRef))
        (Transformation|AddLocalRotation (Variables|Default|GetSmall) (Math|Rotator|MakeRotator 0.0 _speedtick_2 0.0) false false)
        (Transformation|AddLocalRotation (Variables|Default|GetBig) (Math|Rotator|MakeRotator 0.0 (* _speedtick_2 -1.2e+02) 0.0) false false)
        (else
          (Transformation|AddLocalRotation (Variables|Default|GetSmall) (Math|Rotator|MakeRotator 0.0 _speedtick 0.0) false false)
          (Transformation|AddLocalRotation (Variables|Default|GetBig) (Math|Rotator|MakeRotator 0.0 (* _speedtick 12.0) 0.0) false false))))
    (:then_1
      (Utilities|FlowControl|DoOnce false
        (:Completed
          (Utilities|FlowControl|Delay 0.9)
          (bind _returnvalue (Audio|SpawnSoundatLocation (Variables|Default|GetSoundClock) (Transformation|GetWorldLocation (Variables|Default|GetBase)) "0, 0, 0" 1.0 1.0 0.0 0 0)))))))

(fn ConstructionScript)