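; BP_Radio is a radio prop for motion-controller play that plays a sound cue and goes silent while the player is rewinding.
; Every tick it reads the player pawn's RewindState, stopping the audio during rewind and otherwise spawning a new attached sound whenever playback has stopped.
; GetSocketName picks a left- or right-hand "TakeRadio" socket based on the pawn's GrabLeft flag.
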(event EventBeginPlay
  (|CallParentFunction)
  (Variables|Default|SetRadioLocation (Transformation|GetWorldLocation (Variables|Default|GetStaticMesh))))

(event Collision|EventActorBeginOverlap
  (params (OtherActor :type Actor%20Object%20Reference))
  (|CallParentFunction OtherActor) ; This node is disabled and will not be called.\nDrag off pins to build functionality.
)

(event EventTick
  (params (DeltaSeconds :type Float%20%28single-precision%29))
  (|CallParentFunction DeltaSeconds)
  (bind _asmotion_controller_pawn (Utilities|Casting|CastToMotionControllerPawn (Game|Player|GetPlayerPawn 0)))
  (if (Variables|/Game/Blueprint/MotionControllerPawn.MotionControllerPawn_C|GetRewindState _asmotion_controller_pawn)
    (Utilities|IsValid (Variables|Default|GetAttachedSound)
      (:Is%20Valid
        (Audio|Components|Audio|Stop (Variables|Default|GetSC_Radio)))
      (:Is%20Not%20Valid
        (Audio|Components|Audio|Stop (Variables|Default|GetSC_Radio))))
    (else
      (Utilities|IsValid (Variables|Default|GetAttachedSound)
        (:Is%20Valid
          (if (not (Audio|Components|Audio|IsPlaying (Variables|Default|GetAttachedSound)))
            (bind _returnvalue (Audio|SpawnSoundAttached "/Game/Sounds/SC_Radio.SC_Radio" (Variables|Default|GetSC_Radio) "None" (Variables|Default|GetRadioLocation) "0, 0, 0" "KeepRelativeOffset" false 1.0 1.0 0.0 0 0 :!label _label))
            (bind _output_get (Variables|Default|SetAttachedSound _returnvalue))
            (if (not (Audio|Components|Audio|IsPlaying _output_get))
              (Audio|Components|Audio|Play (Variables|Default|GetAttachedSound) 0.0))))
        (:Is%20Not%20Valid
          (if (not (Audio|Components|Audio|IsPlaying (Variables|Default|GetSC_Radio)))
            (goto _label)))))))

(fn ConstructionScript
  (|CallParentFunction))

(fn GetSocketName
  (bind _asmotion_controller_pawn (Utilities|Casting|CastToMotionControllerPawn (Game|Player|GetPlayerPawn 0)))
  (if (Variables|/Game/Blueprint/MotionControllerPawn.MotionControllerPawn_C|GetGrabLeft _asmotion_controller_pawn)
    (LocalVariables|SetSocketName (Utilities|String|StringToName (Utilities|String|Append "TakeRadio" "_L")))
    (else
      (LocalVariables|SetSocketName (Utilities|String|StringToName (Utilities|String|Append "TakeRadio" "_R")))))
  (return (LocalVariables|GetSocketName)))