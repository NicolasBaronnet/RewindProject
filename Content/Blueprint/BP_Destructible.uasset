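; BP_Destructible is an object that breaks when struck hard enough by a BP_Hammer and is restored during rewind.
; A Box overlap checks the hammer's speed against DestructionThreshold, then hides the still-visible StaticMesh, calls CallActivateButton and plays a glass-breaking sound at the mesh.
; Breaking only toggles visibility, so Tick restores the object by showing the mesh whenever TimerRef's RewindStateRef is true.
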(event OnComponentBeginOverlap(Box)
  (params (OverlappedComponent :type Primitive%20Component%20Object%20Reference) (OtherActor :type Actor%20Object%20Reference) (OtherComp :type Primitive%20Component%20Object%20Reference) (OtherBodyIndex :type Integer) (bFromSweep :type Boolean) (SweepResult :type Hit%20Result%20Structure%20%28by%20ref%29))
  (if (Rendering|IsVisible (Variables|Default|GetStaticMesh))
    (bind _asbp_hammer (Utilities|Casting|CastToBP_Hammer OtherActor))
    (if (> (Variables|/Game/Blueprint/BP_Hammer.BP_Hammer_C|GetSpeed _asbp_hammer) (Variables|Default|GetDestructionThreshold))
      (Rendering|SetVisibility (Variables|Default|GetStaticMesh) false false)
      (Default|CallActivateButton)
      (Audio|PlaySoundatLocation "/Game/Sounds/Ambiant/glass_breaking.glass_breaking" (Transformation|GetWorldLocation (Variables|Default|GetStaticMesh)) "0, 0, 0" 1.0 1.0 0.0 0 0 0))))

(event EventBeginPlay)

(event Collision|EventActorBeginOverlap
  (params (OtherActor :type Actor%20Object%20Reference)))

(event EventTick
  (params (DeltaSeconds :type Float%20%28single-precision%29))
  (if (Variables|/Game/Blueprint/BP_Timer.BP_Timer_C|GetRewindStateRef (Variables|Default|GetTimerRef))
    (Rendering|SetVisibility (Variables|Default|GetStaticMesh) true false)))

(fn ConstructionScript)