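; BP_Smoke is a smoke actor that appears at a set point on a timer and can be cleared by a button.
; Tick reveals the smoke through a DoOnce once the timer's time drops to SpawnTimer or below, toggling its activation the first time only.
; The bound button event hides the smoke and plays a wind sound.
; During rewind, Tick stops that sound, hides the smoke and resets the DoOnce so it can reappear.
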(event Custom|DisableSmoke
  (bind _returnvalue (Audio|SpawnSoundatLocation (Variables|Default|GetWindRef) "0, 0, 0" "0, 0, 0" 1.0 1.0 0.0 0 0))
  (Rendering|SetVisibility (Variables|Default|GetSmoke) false true))

(event EventBeginPlay
  (EventDispatchers|BindEventtoSmokeDisable (Variables|Default|GetButtonRef) (delegate Custom|DisableSmoke)))

(event Collision|EventActorBeginOverlap
  (params (OtherActor :type Actor%20Object%20Reference)))

(event EventTick
  (params (DeltaSeconds :type Float%20%28single-precision%29))
  (bind _smoke (Variables|Default|GetSmoke))
  (if (Variables|/Game/Blueprint/BP_Timer.BP_Timer_C|GetRewindStateRef (Variables|Default|GetTimerRef))
    (Utilities|IsValid (stale Custom|DisableSmoke _returnvalue)
      (:Is%20Valid
        (Audio|Components|Audio|Stop (stale Custom|DisableSmoke _returnvalue)))
      (:Is%20Not%20Valid
        _))
    (Rendering|SetVisibility (Variables|Default|GetSmoke) false true)
    (goto _label Reset)
    (elif (<= (Variables|/Game/Blueprint/BP_Timer.BP_Timer_C|GetTime (Variables|Default|GetTimerRef)) (Variables|Default|GetSpawnTimer))
      (Utilities|FlowControl|DoOnce false :!label _label
        (:Completed
          (Utilities|FlowControl|Sequence
            (:then_0
              (Utilities|FlowControl|DoOnce false
                (:Completed
                  (Components|Activation|ToggleActive _smoke))))
            (:then_1
              (Rendering|SetVisibility _smoke true true))))))))

(fn ConstructionScript)