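; BP_ColorPanelCover is a cover for a color panel that slides aside when triggered.
; On BeginPlay it binds MovePanel to the phone base's CodeBon event and the timer's FlipColorPanel event.
; Once triggered, Tick nudges the static mesh along negative world X each frame until it reaches a fixed limit, without delta-time scaling.
; The timer's rewind state cancels the movement.
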(event Custom|MovePanel
  (Variables|Default|SetTranslate true))

(event EventBeginPlay
  (|CallParentFunction)
  (EventDispatchers|BindEventtoCodeBon (Variables|Default|GetPhoneBaseRef) (delegate Custom|MovePanel))
  (EventDispatchers|BindEventtoFlipColorPanel (Variables|Default|GetTimerRef) (delegate Custom|MovePanel)))

(event Collision|EventActorBeginOverlap
  (params (OtherActor :type Actor%20Object%20Reference)))

(event EventTick
  (params (DeltaSeconds :type Float%20%28single-precision%29))
  (|CallParentFunction DeltaSeconds)
  (if (Variables|/Game/Blueprint/BP_Timer.BP_Timer_C|GetRewindStateRef (Variables|Default|GetTimerRef))
    (Variables|Default|SetTranslate false)
    (elif (Variables|Default|GetTranslate)
      (if (> (.x (Transformation|GetWorldLocation (Variables|Default|GetStaticMesh))) -3e+01)
        (Transformation|AddWorldOffset (Variables|Default|GetStaticMesh) (Math|Vector|MakeVector -1.0 0.0 0.0) false false)
        (Variables|Default|SetTranslate true)
        (else
          (Variables|Default|SetTranslate false))))))

(fn ConstructionScript
  (|CallParentFunction))