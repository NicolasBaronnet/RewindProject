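; BP_ButtonBase is a button actor that reacts when something enters or leaves its sphere trigger.
; For the first TypeBouton value, overlap snaps the mesh to the End component's relative location and calls ButtonActivated; the second type has no behavior here.
; Ending overlap returns the mesh to the Start location for any type, and neither overlap event filters which actor triggers it.
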(event OnComponentEndOverlap(Sphere)
  (params (OverlappedComponent :type Primitive%20Component%20Object%20Reference) (OtherActor :type Actor%20Object%20Reference) (OtherComp :type Primitive%20Component%20Object%20Reference) (OtherBodyIndex :type Integer))
  (Transformation|SetRelativeLocation (Variables|Default|GetStaticMesh) (Variables|/Script/Engine.SceneComponent|GetRelativeLocation (Variables|Default|GetStart)) false false))

(event OnComponentBeginOverlap(Sphere)
  (params (OverlappedComponent :type Primitive%20Component%20Object%20Reference) (OtherActor :type Actor%20Object%20Reference) (OtherComp :type Primitive%20Component%20Object%20Reference) (OtherBodyIndex :type Integer) (bFromSweep :type Boolean) (SweepResult :type Hit%20Result%20Structure%20%28by%20ref%29))
  (if (Utilities|Enum|Equal(Enum) (Variables|Default|GetTypeBouton) "NewEnumerator0")
    (Transformation|SetRelativeLocation (Variables|Default|GetStaticMesh) (Variables|/Script/Engine.SceneComponent|GetRelativeLocation (Variables|Default|GetEnd)) false false)
    (Default|CallButtonActivated)
    (elif (Utilities|Enum|Equal(Enum) (Variables|Default|GetTypeBouton) "NewEnumerator1")
      _)))

(event EventBeginPlay)

(event Collision|EventActorBeginOverlap
  (params (OtherActor :type Actor%20Object%20Reference)))

(event EventTick
  (params (DeltaSeconds :type Float%20%28single-precision%29)))

(fn ConstructionScript)