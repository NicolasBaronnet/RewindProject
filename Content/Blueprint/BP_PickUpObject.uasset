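; BP_PickUpObject is an actor that can be picked up, carried on another component and dropped.
; Pickup turns off the static mesh's physics, then snaps both the root and the mesh to the given component while keeping world scale.
; Drop re-enables physics and detaches both components.
; GetSocketName supplies the attach socket (None here), and GrabBehvior returns a fixed grab-behavior enum value.
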(event EventBeginPlay
  (|CallParentFunction) ; This node is disabled and will not be called.\nDrag off pins to build functionality.
)

(event Collision|EventActorBeginOverlap
  (params (OtherActor :type Actor%20Object%20Reference)))

(event EventTick
  (params (DeltaSeconds :type Float%20%28single-precision%29))
  (|CallParentFunction DeltaSeconds))

(event EventPickup
  (params (AttachTo :type Scene%20Component%20Object%20Reference))
  (Physics|SetSimulatePhysics (Variables|Default|GetStaticMesh) false)
  (bind _socket (CallFunction|GetSocketName))
  (Transformation|AttachComponentToComponent (Variables|Default|GetDefaultSceneRoot) AttachTo _socket "SnapToTarget" "SnapToTarget" "KeepWorld" false)
  (Transformation|AttachComponentToComponent (Variables|Default|GetStaticMesh) AttachTo _socket "SnapToTarget" "SnapToTarget" "KeepWorld" false))

(event EventDrop
  (Physics|SetSimulatePhysics (Variables|Default|GetStaticMesh) true)
  (Transformation|DetachFromComponent (Variables|Default|GetStaticMesh) "KeepRelative" "KeepRelative" "KeepRelative" true)
  (Transformation|DetachFromComponent (Variables|Default|GetDefaultSceneRoot) "KeepRelative" "KeepRelative" "KeepRelative" true))

(fn ConstructionScript
  (|CallParentFunction))

(fn GetSocketName
  (return "None"))

(fn GrabBehvior
  (return "NewEnumerator0"))