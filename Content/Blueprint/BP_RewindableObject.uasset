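; BP_RewindableObject is a physics object that rewinds its motion while the player's MotionControllerPawn has RewindState on.
; Each tick it records the static mesh's world transform and velocities into two arrays, dropping the oldest entries at MaxIndex.
; During rewind it pops the newest entries, teleporting the mesh and restoring velocities, holding on the last remaining one.
; VelocityArray packs linear velocity into a transform's Location and angular velocity into its Scale.
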(event EventBeginPlay
  (bind _asmotion_controller_pawn (Utilities|Casting|CastToMotionControllerPawn (Game|Player|GetPlayerPawn 0)))
  (Variables|Default|SetCharacterRef _asmotion_controller_pawn))

(event EventTick
  (params (DeltaSeconds :type Float%20%28single-precision%29))
  (bind _staticmesh (Variables|Default|GetStaticMesh))
  (bind _velocityarray (Variables|Default|GetVelocityArray))
  (bind _velocityarray_2 (Variables|Default|GetVelocityArray))
  (bind _returnvalue (Utilities|Array|LastIndex _velocityarray))
  (bind _returnvalue_2 (Utilities|Array|LastIndex _velocityarray_2))
  (bind _output (Utilities|Array|Get(acopy) _velocityarray _returnvalue))
  (bind (_location _rotation _scale) (Math|Transform|BreakTransform _output))
  (Utilities|FlowControl|Sequence
    (:then_0
      (if (Variables|/Game/Blueprint/MotionControllerPawn.MotionControllerPawn_C|GetRewindState (Variables|Default|GetCharacterRef))
        (bind _output_get (Variables|Default|SetLastIndex (Utilities|Array|LastIndex (Variables|Default|GetTransformArray))))
        (Transformation|SetWorldTransform (Variables|Default|GetStaticMesh) (Utilities|Array|Get(acopy) (Variables|Default|GetTransformArray) _output_get) false true)
        (if (> (Variables|Default|GetLastIndex) 0)
          (Utilities|Array|RemoveIndex (Variables|Default|GetTransformArray) (Variables|Default|GetLastIndex)))
        (else
          (Utilities|Array|Add (Variables|Default|GetTransformArray) (Transformation|GetWorldTransform (Variables|Default|GetStaticMesh))))))
    (:then_1
      (if (>= (Utilities|Array|Length (Variables|Default|GetTransformArray)) (Variables|Default|GetMaxIndex))
        (Utilities|Array|RemoveIndex (Variables|Default|GetTransformArray))
        (Utilities|Array|RemoveIndex (Variables|Default|GetVelocityArray))))
    (:then_2
      (if (Variables|/Game/Blueprint/MotionControllerPawn.MotionControllerPawn_C|GetRewindState (Variables|Default|GetCharacterRef))
        (Physics|SetPhysicsLinearVelocity (Variables|Default|GetStaticMesh) _location false "None")
        (Class|PrimitiveComponent|SetPhysicsAngularVelocityinDegrees (Variables|Default|GetStaticMesh) _scale false "None")
        (if (> _returnvalue_2 0)
          (Utilities|Array|RemoveIndex (Variables|Default|GetVelocityArray) _returnvalue_2))
        (else
          (bind _returnvalue_3 (Physics|GetPhysicsLinearVelocity _staticmesh "None"))
          (Utilities|Array|Add (Variables|Default|GetVelocityArray) (Math|Transform|MakeTransform _returnvalue_3 "0, 0, 0" (Physics|GetPhysicsAngularVelocityinDegrees _staticmesh "None"))))))))

(fn ConstructionScript)