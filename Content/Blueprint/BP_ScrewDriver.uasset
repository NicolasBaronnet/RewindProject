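; BP_ScrewDriver is a screwdriver Blueprint for a motion-controller setup that supplies the socket name to use when it is taken.
; GetSocketName casts the player pawn to MotionControllerPawn and reads GrabLeft to build a TakeScrewDriver socket name with a left or right hand suffix.
; The event graph holds only disabled default events, and the construction script only calls its parent.
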(event EventBeginPlay
  (|CallParentFunction) ; This node is disabled and will not be called.\nDrag off pins to build functionality.
)

(event Collision|EventActorBeginOverlap
  (params (OtherActor :type Actor%20Object%20Reference))
  (|CallParentFunction OtherActor) ; This node is disabled and will not be called.\nDrag off pins to build functionality.
)

(event EventTick
  (params (DeltaSeconds :type Float%20%28single-precision%29))
  (|CallParentFunction DeltaSeconds) ; This node is disabled and will not be called.\nDrag off pins to build functionality.
)

(fn ConstructionScript
  (|CallParentFunction))

(fn GetSocketName
  (bind _asmotion_controller_pawn (Utilities|Casting|CastToMotionControllerPawn (Game|Player|GetPlayerPawn 0)))
  (if (Variables|/Game/Blueprint/MotionControllerPawn.MotionControllerPawn_C|GetGrabLeft _asmotion_controller_pawn)
    (LocalVariables|SetSocketName (Utilities|String|StringToName (Utilities|String|Append "TakeScrewDriver" "_L")))
    (return (LocalVariables|GetSocketName))
    (else
      (LocalVariables|SetSocketName (Utilities|String|StringToName (Utilities|String|Append "TakeScrewDriver" "_R"))))))