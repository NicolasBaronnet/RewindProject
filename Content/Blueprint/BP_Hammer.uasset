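; BP_Hammer is a hammer actor for VR that tracks its own movement speed and supplies a hand-specific grab socket.
; Tick derives Speed from the root's world-space displacement over delta time, then stores the new Position, skipping updates at the world origin.
; GetSocketName checks GrabLeft on the player's MotionControllerPawn to return the left or right TakeHammer socket name.
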(event EventBeginPlay
  (|CallParentFunction) ; This node is disabled and will not be called.\nDrag off pins to build functionality.
)

(event Collision|EventActorBeginOverlap
  (params (OtherActor :type Actor%20Object%20Reference))
  (|CallParentFunction OtherActor) ; This node is disabled and will not be called.\nDrag off pins to build functionality.
)

(event EventTick
  (params (DeltaSeconds :type Float%20%28single-precision%29))
  (bind _defaultsceneroot (Variables|Default|GetDefaultSceneRoot))
  (bind _returnvalue (Transformation|GetWorldLocation _defaultsceneroot))
  (|CallParentFunction DeltaSeconds)
  (if (Class|KismetMathLibrary|NotEqualExactlyVectorVector _returnvalue "0, 0, 0")
    (Variables|Default|SetSpeed (/ (Math|Vector|VectorLength (- (Variables|Default|GetPosition) _returnvalue)) DeltaSeconds))
    (Variables|Default|SetPosition (Transformation|GetWorldLocation (Variables|Default|GetDefaultSceneRoot)))))

(fn ConstructionScript
  (|CallParentFunction))

(fn GetSocketName
  (bind _asmotion_controller_pawn (Utilities|Casting|CastToMotionControllerPawn (Game|Player|GetPlayerPawn 0)))
  (if (Variables|/Game/Blueprint/MotionControllerPawn.MotionControllerPawn_C|GetGrabLeft _asmotion_controller_pawn)
    (LocalVariables|SetSocketName (Utilities|String|StringToName (Utilities|String|Append "TakeHammer" "_L")))
    (else
      (LocalVariables|SetSocketName (Utilities|String|StringToName (Utilities|String|Append "TakeHammer" "_R")))))
  (return (LocalVariables|GetSocketName)))