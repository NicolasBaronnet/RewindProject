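; BP_Alarm is an alarm actor with a spotlight that spins to act as a rotating warning light.
; Each Tick yaws the light by RotationSpeed, or backwards at double speed while TimerRef reports a rewind state, with no delta-time scaling.
; On BeginPlay it binds to BombRef's winning event, which zeroes RotationSpeed and stops the spin.
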(event Custom|WinningLane
  (Variables|Default|SetRotationSpeed 0.0))

(event EventBeginPlay
  (EventDispatchers|BindEventtoWinningEvent (Variables|Default|GetBombRef) (delegate Custom|WinningLane)))

(event Collision|EventActorBeginOverlap
  (params (OtherActor :type Actor%20Object%20Reference)))

(event EventTick
  (params (DeltaSeconds :type Float%20%28single-precision%29))
  (if (Variables|/Game/Blueprint/BP_Timer.BP_Timer_C|GetRewindStateRef (Variables|Default|GetTimerRef))
    (Transformation|AddLocalRotation (Variables|Default|GetSpotLight) (Math|Rotator|MakeRotator 0.0 0.0 (* -2 (Variables|Default|GetRotationSpeed))) false false)
    (else
      (Transformation|AddLocalRotation (Variables|Default|GetSpotLight) (Math|Rotator|MakeRotator 0.0 0.0 (Variables|Default|GetRotationSpeed)) false false))))

(fn ConstructionScript)