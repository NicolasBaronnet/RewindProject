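; Base pickup actor that BP_MotionController can grab, attach to itself and drop.
; Pickup turns off mesh physics and snaps the root to the given component at the socket from GetSocketName, which returns None here.
; Drop re-enables physics and detaches in world space.
; StartUse only prints a debug string, and GrabBehvior returns a fixed enum value.
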(event EventBeginPlay)

(event Collision|EventActorBeginOverlap
  (params (OtherActor :type Actor%20Object%20Reference)))

(event EventTick
  (params (DeltaSeconds :type Float%20%28single-precision%29)))

(event EventPickup
  (params (AttachTo :type Scene%20Component%20Object%20Reference))
  (Physics|SetSimulatePhysics (Variables|Debug|GetStaticMeshComponent) false)
  (bind _socket (CallFunction|GetSocketName))
  (Transformation|AttachComponentToComponent (VehicleSound|GetRootComponent) AttachTo _socket "SnapToTarget" "SnapToTarget" "KeepRelative" false))

(event EventDrop
  (Physics|SetSimulatePhysics (Variables|Debug|GetStaticMeshComponent) true)
  (Transformation|DetachFromActor "KeepWorld" "KeepWorld" "KeepWorld"))

(event EventStartUse
  (Development|PrintString "using"))

(fn ConstructionScript)

(fn GetSocketName
  (return ""))

(fn GrabBehvior
  (return "NewEnumerator0"))