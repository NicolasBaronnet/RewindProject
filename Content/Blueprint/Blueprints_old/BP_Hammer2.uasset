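; BP_Hammer2 is a hammer actor that tracks its own movement speed.
; Each tick it derives Speed from the distance its static mesh moved since the stored Position, divided by delta time, then updates Position.
; The update is skipped while the mesh sits at world origin.
; GetSocketName returns the fixed "TakeHammer" socket name; BeginPlay and overlap events are unused stubs.
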(event EventBeginPlay
  (|CallParentFunction) ; This node is disabled and will not be called.\nDrag off pins to build functionality.
)

(event Collision|EventActorBeginOverlap
  (params (OtherActor :type Actor%20Object%20Reference))
  (|CallParentFunction OtherActor) ; This node is disabled and will not be called.\nDrag off pins to build functionality.
)

(event EventTick
  (params (DeltaSeconds :type Float%20%28single-precision%29))
  (bind _staticmeshcomponent (Variables|Default|GetStaticMeshComponent))
  (bind _returnvalue (Transformation|GetWorldLocation _staticmeshcomponent))
  (if (Math|Vector|NotEqual(Vector) _returnvalue "0, 0, 0" 0.0001)
    (Variables|Default|Setspeed (/ (Math|Vector|VectorLength (- (Variables|Default|GetPosition) _returnvalue)) DeltaSeconds))
    (Variables|Default|SetPosition (Transformation|GetWorldLocation (Variables|Default|GetStaticMeshComponent)))))

(fn ConstructionScript
  (|CallParentFunction))

(fn GetSocketName
  (return "TakeHammer"))