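; BP_ColorPanel is a VR four-colour code panel that prints an "electricity cut" message when the entered sequence matches TrueCode.
; Red, Blue, Green and Yellow box overlaps append names to ButtonName, debounced by DoOnce until overlap ends, restarting once CodeLenght reaches three.
; Tick compares the string with TrueCode.
; BeginPlay caches the pawn's controllers in HandCollisions, looping until found, but overlaps never check them; ButtonFunction is empty.
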(event OnComponentBeginOverlap(RedBox)
  (params (OverlappedComponent :type Primitive%20Component%20Object%20Reference) (OtherActor :type Actor%20Object%20Reference) (OtherComp :type Primitive%20Component%20Object%20Reference) (OtherBodyIndex :type Integer) (bFromSweep :type Boolean) (SweepResult :type Hit%20Result%20Structure%20%28by%20ref%29))
  (Utilities|FlowControl|DoOnce false
    (:Completed
      (if (< (Variables|Default|GetCodeLenght) 3)
        (Variables|Default|SetButtonName (Utilities|String|Append (Variables|Default|GetButtonName) "Red"))
        (Math|Integer|IncrementInt (Variables|Default|GetCodeLenght)
          (:%20%20
            (Development|PrintString (Variables|Default|GetButtonName))))
        (else
          (Variables|Default|SetButtonName "Red")
          (Variables|Default|SetCodeLenght 0))))))

(event OnComponentEndOverlap(RedBox)
  (params (OverlappedComponent :type Primitive%20Component%20Object%20Reference) (OtherActor :type Actor%20Object%20Reference) (OtherComp :type Primitive%20Component%20Object%20Reference) (OtherBodyIndex :type Integer))
  (Utilities|FlowControl|DoOnce false) ; enters at Reset
)

(event OnComponentBeginOverlap(BlueBox)
  (params (OverlappedComponent :type Primitive%20Component%20Object%20Reference) (OtherActor :type Actor%20Object%20Reference) (OtherComp :type Primitive%20Component%20Object%20Reference) (OtherBodyIndex :type Integer) (bFromSweep :type Boolean) (SweepResult :type Hit%20Result%20Structure%20%28by%20ref%29))
  (Utilities|FlowControl|DoOnce false
    (:Completed
      (if (< (Variables|Default|GetCodeLenght) 3)
        (Variables|Default|SetButtonName (Utilities|String|Append (Variables|Default|GetButtonName) "Blue"))
        (Math|Integer|IncrementInt (Variables|Default|GetCodeLenght)
          (:%20%20
            (Development|PrintString (Variables|Default|GetButtonName))))
        (else
          (Variables|Default|SetButtonName "Blue")
          (Variables|Default|SetCodeLenght 0))))))

(event OnComponentEndOverlap(BlueBox)
  (params (OverlappedComponent :type Primitive%20Component%20Object%20Reference) (OtherActor :type Actor%20Object%20Reference) (OtherComp :type Primitive%20Component%20Object%20Reference) (OtherBodyIndex :type Integer))
  (Utilities|FlowControl|DoOnce false) ; enters at Reset
)

(event OnComponentBeginOverlap(GreenBox)
  (params (OverlappedComponent :type Primitive%20Component%20Object%20Reference) (OtherActor :type Actor%20Object%20Reference) (OtherComp :type Primitive%20Component%20Object%20Reference) (OtherBodyIndex :type Integer) (bFromSweep :type Boolean) (SweepResult :type Hit%20Result%20Structure%20%28by%20ref%29))
  (Utilities|FlowControl|DoOnce false
    (:Completed
      (if (< (Variables|Default|GetCodeLenght) 3)
        (Variables|Default|SetButtonName (Utilities|String|Append (Variables|Default|GetButtonName) "Green"))
        (Math|Integer|IncrementInt (Variables|Default|GetCodeLenght)
          (:%20%20
            (Development|PrintString (Variables|Default|GetButtonName))))
        (else
          (Variables|Default|SetButtonName "Green")
          (Variables|Default|SetCodeLenght 0))))))

(event OnComponentEndOverlap(GreenBox)
  (params (OverlappedComponent :type Primitive%20Component%20Object%20Reference) (OtherActor :type Actor%20Object%20Reference) (OtherComp :type Primitive%20Component%20Object%20Reference) (OtherBodyIndex :type Integer))
  (Utilities|FlowControl|DoOnce false) ; enters at Reset
)

(event OnComponentBeginOverlap(YellowBox)
  (params (OverlappedComponent :type Primitive%20Component%20Object%20Reference) (OtherActor :type Actor%20Object%20Reference) (OtherComp :type Primitive%20Component%20Object%20Reference) (OtherBodyIndex :type Integer) (bFromSweep :type Boolean) (SweepResult :type Hit%20Result%20Structure%20%28by%20ref%29))
  (Utilities|FlowControl|DoOnce false
    (:Completed
      (if (< (Variables|Default|GetCodeLenght) 3)
        (Variables|Default|SetButtonName (Utilities|String|Append (Variables|Default|GetButtonName) "Yellow"))
        (Math|Integer|IncrementInt (Variables|Default|GetCodeLenght)
          (:%20%20
            (Development|PrintString (Variables|Default|GetButtonName))))
        (else
          (Variables|Default|SetButtonName "Yellow")
          (Variables|Default|SetCodeLenght 0))))))

(event OnComponentEndOverlap(YellowBox)
  (params (OverlappedComponent :type Primitive%20Component%20Object%20Reference) (OtherActor :type Actor%20Object%20Reference) (OtherComp :type Primitive%20Component%20Object%20Reference) (OtherBodyIndex :type Integer))
  (Utilities|FlowControl|DoOnce false) ; enters at Reset
)

(event EventBeginPlay
  (bind _asmotion_controller_pawn (Utilities|Casting|CastToMotionControllerPawnClass "/Game/Blueprint/MotionControllerPawn.MotionControllerPawn_C" :!label _label))
  (bind _returnvalue (Actor|GetActorOfClass _asmotion_controller_pawn))
  (Utilities|IsValid _returnvalue
    (:Is%20Valid
      (Utilities|Array|Add (Variables|Default|GetHandCollisions) (Variables|/Game/Blueprint/MotionControllerPawn.MotionControllerPawn_C|GetLeftController _returnvalue))
      (Utilities|Array|Add (Variables|Default|GetHandCollisions) (Variables|/Game/Blueprint/MotionControllerPawn.MotionControllerPawn_C|GetRightController _returnvalue)))
    (:Is%20Not%20Valid
      (goto _label))))

(event Collision|EventActorBeginOverlap
  (params (OtherActor :type Actor%20Object%20Reference)))

(event EventTick
  (params (DeltaSeconds :type Float%20%28single-precision%29))
  (if (Utilities|Enum|Equal(Enum) (Variables|Default|GetButtonName) (Variables|Default|GetTrueCode))
    (Utilities|FlowControl|DoOnce false :!label _label
      (:Completed
        (Development|PrintString "electricité coupée")))
    (else
      (goto _label Reset))))

(fn ConstructionScript)

(fn ButtonFunction
  (params (ButtonColor :type String) (OverlappedActor :type Actor%20Object%20Reference)))