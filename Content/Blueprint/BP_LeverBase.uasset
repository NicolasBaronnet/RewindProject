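; BP_LeverBase is a grabbable lever base that follows the gripping hand and signals when it is pulled past a threshold.
; Each TickGrip pitches RotationPoint toward the hand using a look-at rotation, forcing world roll and yaw to zero without clamping.
; The LeverIsActive dispatcher fires on every grip tick at or above the pitch threshold.
; Grab and Release are empty, and GrabBehvior returns a fixed grab type.
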(event EventBeginPlay
  (|CallParentFunction) ; This node is disabled and will not be called.\nDrag off pins to build functionality.
)

(event Collision|EventActorBeginOverlap
  (params (OtherActor :type Actor%20Object%20Reference))
  (|CallParentFunction OtherActor) ; This node is disabled and will not be called.\nDrag off pins to build functionality.
)

(event EventTick
  (params (DeltaSeconds :type Float%20%28single-precision%29))
  (|CallParentFunction DeltaSeconds) ; This node is disabled and will not be called.\nDrag off pins to build functionality.
)

(event EventGrab)

(event EventRelease)

(event EventTickGrip
  (params (HandTransform :type Transform))
  (bind _location (Math|Transform|BreakTransform HandTransform))
  (bind _rotationpoint (Variables|Default|GetRotationPoint))
  (bind _returnvalue (Transformation|GetWorldLocation _rotationpoint))
  (bind _returnvalue_2 (Math|Rotator|FindLookatRotation _returnvalue _location))
  (bind _pitch (Math|Rotator|BreakRotator _returnvalue_2))
  (Transformation|SetWorldRotation _rotationpoint (Math|Rotator|MakeRotator 0.0 _pitch 0.0) false false)
  (if (>= _pitch (Variables|Default|GetThreshold))
    (Default|CallLeverIsActive)))

(fn ConstructionScript
  (|CallParentFunction))

(fn GrabBehvior
  (return "NewEnumerator1"))