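; BP_Lights controls the desk, main and ambient lights, cutting power when a drawer unlocks.
; BeginPlay binds SetallLightinactive to the color panel's unlocked-drawer event.
; That event zeroes all intensities and plays a shutdown sound, then an unlock sound after a short Delay, all wired inside the main-light loop.
; Tick reapplies lit intensities every frame while the timer's rewind state is true.
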(event Custom|Set%20all%20Light%20inactive
  (Rendering|Components|Light|SetIntensity (Variables|/Game/Blueprint/BP_Desklight.BP_Desklight_C|GetPointLight (Variables|Default|GetDeskLight)) 0.0)
  (for _array_element (Variables|Default|GetMainLight)
    (Rendering|Components|Light|SetIntensity (Variables|/Script/Engine.Light|GetLightComponent _array_element) 0.0)
    (Rendering|Components|Light|SetIntensity (Variables|/Script/Engine.Light|GetLightComponent (Variables|Default|GetAmbientLight)) 0.0)
    (Audio|PlaySound2D "/Game/Sounds/Ambiant/power_shutDown.power_shutDown" 1.0 1.0 0.0 0 0)
    (Utilities|FlowControl|Delay 0.5)
    (Audio|PlaySound2D "/Game/Sounds/Ambiant/unlock.unlock" 1.0 1.0 0.0 0 0)))

(event EventBeginPlay
  (EventDispatchers|BindEventtoUnlockedDrawer (Variables|Default|GetColorPanelRef) (delegate Custom|Set%20all%20Light%20inactive)))

(event Collision|EventActorBeginOverlap
  (params (OtherActor :type Actor%20Object%20Reference)))

(event EventTick
  (params (DeltaSeconds :type Float%20%28single-precision%29))
  (if (Variables|/Game/Blueprint/BP_Timer.BP_Timer_C|GetRewindStateRef (Variables|Default|GetTimerRef))
    (Rendering|Components|Light|SetIntensity (Variables|/Game/Blueprint/BP_Desklight.BP_Desklight_C|GetPointLight (Variables|Default|GetDeskLight)) (Variables|Default|GetDeskLightIntensity))
    (for _array_element (Variables|Default|GetMainLight)
      (Rendering|Components|Light|SetIntensity (Variables|/Script/Engine.Light|GetLightComponent _array_element) (Variables|Default|GetMainLightIntensity))
      (Rendering|Components|Light|SetIntensity (Variables|/Script/Engine.Light|GetLightComponent (Variables|Default|GetAmbientLight)) 0.1))))

(fn ConstructionScript)