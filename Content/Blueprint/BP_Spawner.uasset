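; Spawner actor that creates a BP_PickupBase cube whenever one of its linked buttons is activated.
; On BeginPlay it binds SpawnCube to the activation event of every entry in ButtonList.
; Each call spawns the pickup at the Spawnpoint component's world transform, ignoring collisions, then increments the CptCube counter and prints it.
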(event Custom|SpawnCube
  (Game|SpawnActorfromClass "/Game/Blueprint/Blueprints_old/BP_PickupBase.BP_PickupBase_C" (Transformation|GetWorldTransform (Variables|Default|GetSpawnpoint)) "AlwaysSpawn" 0 0)
  (bind _result (Math|Integer|IncrementInt (Variables|Default|GetCptCube))
    (:%20%20
      (Development|PrintString (Utilities|String|ToString(Integer) _result)))))

(event EventBeginPlay
  (for _array_element (Variables|Default|GetButtonList)
    (EventDispatchers|BindEventtoButtonActivated _array_element (delegate Custom|SpawnCube))))

(event Collision|EventActorBeginOverlap
  (params (OtherActor :type Actor%20Object%20Reference)))

(event EventTick
  (params (DeltaSeconds :type Float%20%28single-precision%29)))

(fn ConstructionScript)