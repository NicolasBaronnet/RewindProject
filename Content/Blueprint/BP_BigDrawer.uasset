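; BP_BigDrawer is a drawer Blueprint that extends its parent's behavior with a lock indicator reflecting rewind and lock state.
; Each Tick runs the parent logic, then turns the indicator red and resets a DoOnce while the referenced timer's rewind state is active.
; Outside rewind, an unlocked drawer fires that DoOnce, switching the indicator to green only once until the next rewind.
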(event EventBeginPlay
  (|CallParentFunction) ; This node is disabled and will not be called.\nDrag off pins to build functionality.
)

(event Collision|EventActorBeginOverlap
  (params (OtherActor :type Actor%20Object%20Reference))
  (|CallParentFunction OtherActor) ; This node is disabled and will not be called.\nDrag off pins to build functionality.
)

(event EventTick
  (params (DeltaSeconds :type Float%20%28single-precision%29))
  (|CallParentFunction DeltaSeconds)
  (if (Variables|/Game/Blueprint/BP_Timer.BP_Timer_C|GetRewindStateRef (Variables|Default|GetTimerRefBis))
    (Rendering|Material|SetMaterial (Variables|Default|GetLockedIndic) 0 "/Game/Material/base_content_material/Material_Red.Material_Red")
    (goto _label Reset)
    (elif (not (Variables|Default|GetIsLocked?))
      (Utilities|FlowControl|DoOnce false :!label _label
        (:Completed
          (Rendering|Material|SetMaterial (Variables|Default|GetLockedIndic) 0 "/Game/Material/EASYGRID/M_Grid_Green.M_Grid_Green"))))))

(fn ConstructionScript
  (|CallParentFunction))