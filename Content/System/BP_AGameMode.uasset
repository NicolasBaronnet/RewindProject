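; Game mode Blueprint that creates a UI_Main widget and adds it to the viewport on every Tick, with BeginPlay left empty.
; An unused one-second looping timer is meant to count Timer up, or down while RewindState is set, printing debug values.
; The logic that reads RewindState from MotionControllerPawn and calls TimerFunction is disconnected, and TimerFunction is marked useless.
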(event Custom|Set%20Timer
  (bind _timer (Variables|Default|GetTimer))
  (bind _rewindstate (Variables|Default|GetRewindState))
  ;[1 1 1] Useless
  (Development|PrintString (Utilities|String|ToString(Boolean) _rewindstate))
  (if _rewindstate
    (Math|Float|DecrementFloat _timer
      (:%20%20
        (Development|PrintString (Utilities|String|ToString(Float) _timer))))
    (else
      (Math|Float|IncrementFloat _timer
        (:%20%20
          (Development|PrintString (Utilities|String|ToString(Float) _timer)))))))

(event Custom|TimerFunction
  ;[1 1 1] Useless
  (bind _returnvalue (Utilities|Time|SetTimerbyEvent (delegate Custom|Set%20Timer) 1.0 true))
  (Development|PrintString (Utilities|String|ToString(Float) (Variables|Default|GetTimer))))

(event EventBeginPlay)

(event EventTick
  (params (DeltaSeconds :type Float%20%28single-precision%29))
  (bind _returnvalue (UserInterface|CreateWidget "/Game/UserInterfaces/UI_Main.UI_Main_C"))
  (UserInterface|Viewport|AddtoViewport _returnvalue 0))

(fn ConstructionScript)